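; BP_Grid is a grid actor that builds square, hexagon or triangle tile layouts as instances of one InstancedStaticMesh.
; SpawnGrid clears old instances, takes mesh and material from a shape DataTable, and snaps the center to derive the bottom-left origin.
; Per-shape index math places each tile, staggering hexagons by parity and flipping triangles.
; Optional sphere traces snap tile heights to the ground and skip tiles without hits.
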(event EventBeginPlay)

(event Collision|EventActorBeginOverlap
  (params (OtherActor :type Actor%20Object%20Reference)))

(event EventTick
  (params (DeltaSeconds :type Float%20%28single-precision%29)))

(fn ConstructionScript)

(fn SpawnGrid
  (params (CenterLocation :type Vector) (TileSize :type Vector) (TileCount :type Int%20Point%20Structure) (Shape :type E_Grid_Shape%20Enum :default "NewEnumerator0") (UseEnvironment :type Boolean))
  (bind _returnvalue (CallFunction|GetShapeRowData))
  (bind _instancedstaticmesh (Variables|Default|GetInstancedStaticMesh))
  (bind (_meshsize _mesh _meshmaterial _flatmesh _flatbordermetiral) (Utilities|Struct|BreakS_Grid_Shape_Data _returnvalue))
  (Variables|Default|SetGrid%20Center%20Location CenterLocation)
  (Variables|Default|SetGrid%20Tile%20Size TileSize)
  (Variables|Default|SetGrid%20Shape Shape)
  (Variables|Default|SetGrid%20Tile%20Count TileCount)
  (CallFunction|DeleteGrid)
  ;[1 1 1] 设置gird初始的mesh与material
  (Components|StaticMesh|SetStaticMesh _instancedstaticmesh _flatmesh)
  (Rendering|Material|SetMaterial _instancedstaticmesh 0 _flatbordermetiral)
  (CallFunction|SetGridOffsetfromGround (Variables|Default|GetGridOffsetFromGround))
  ;[1 1 1] 计算出右下角的初始位置与Grid中心位置
  (bind (_centerlocation _bottomleftlocation) (CallFunction|CalCenter&BottomLeftLocation))
  (Variables|Default|SetGrid%20Center%20Location _centerlocation)
  (Variables|Default|SetGridLeftBottomLocation _bottomleftlocation)
  ;[1 1 1] 双层循环嵌套，从起始右下角位置开始，生成地形
  (for _index (range 0 (- (.x (Variables|Default|GetGrid%20Tile%20Count)) 1))
    (LocalVariables|SetX _index)
    (if (Utilities|Enum|NotEqual(Enum) (Variables|Default|GetGrid%20Shape) "NewEnumerator2")
      (for _index_2 (range 0 (- (.y (Variables|Default|GetGrid%20Tile%20Count)) 1))
        (LocalVariables|SetY _index_2)
        (LocalVariables|SetIndex (Utilities|Struct|MakeIntPoint (LocalVariables|GetX) (LocalVariables|GetY)))
        (LocalVariables|SetTileTransform (Math|Transform|MakeTransform (CallFunction|LocationBasedonGridIndex (LocalVariables|GetIndex)) (CallFunction|RotationBasedonGridIndex (LocalVariables|GetIndex)) (/ (Variables|Default|GetGrid%20Tile%20Size) (.MeshSize (Utilities|Struct|BreakS_Grid_Shape_Data (CallFunction|GetShapeRowData))))))
        ;[1 1 1] 选择是否扫描环境
        (if UseEnvironment
          ;[1 1 1] 扫描环境
          (bind (_outlocation _ishitsomething) (CallFunction|TraceforGround (.location (LocalVariables|GetTileTransform))))
          (if _ishitsomething
            (LocalVariables|SetTileTransform (Math|Transform|MakeTransform _outlocation (.rotation (LocalVariables|GetTileTransform)) (.scale (LocalVariables|GetTileTransform))))
            ;[1 1 1] 生成网格
            (Components|InstancedStaticMesh|AddInstance (Variables|Default|GetInstancedStaticMesh) (LocalVariables|GetTileTransform)))
          (else
            ;[1 1 1] 生成网格
            (Components|InstancedStaticMesh|AddInstance (Variables|Default|GetInstancedStaticMesh) (LocalVariables|GetTileTransform)))))
      (else
        (for _index_3 (range (Math|Integer|SelectInt 0 1 (CallFunction|IsIntEven (LocalVariables|GetX))) (- (* (.y (Variables|Default|GetGrid%20Tile%20Count)) 2) 1))
          (LocalVariables|SetY _index_3)
          (Utilities|FlowControl|Sequence
            (:then_1
              (Math|Integer|IncrementInt _index_3
                (:%20%20
                  (LocalVariables|SetIndex (Utilities|Struct|MakeIntPoint (LocalVariables|GetX) (LocalVariables|GetY)))
                  (LocalVariables|SetTileTransform (Math|Transform|MakeTransform (CallFunction|LocationBasedonGridIndex (LocalVariables|GetIndex)) (CallFunction|RotationBasedonGridIndex (LocalVariables|GetIndex)) (/ (Variables|Default|GetGrid%20Tile%20Size) (.MeshSize (Utilities|Struct|BreakS_Grid_Shape_Data (CallFunction|GetShapeRowData))))))
                  (if UseEnvironment
                    (bind (_outlocation_2 _ishitsomething_2) (CallFunction|TraceforGround (.location (LocalVariables|GetTileTransform))))
                    (if _ishitsomething_2
                      (LocalVariables|SetTileTransform (Math|Transform|MakeTransform _outlocation_2 (.rotation (LocalVariables|GetTileTransform)) (.scale (LocalVariables|GetTileTransform))))
                      (Components|InstancedStaticMesh|AddInstance (Variables|Default|GetInstancedStaticMesh) (LocalVariables|GetTileTransform)))
                    (else
                      (Components|InstancedStaticMesh|AddInstance (Variables|Default|GetInstancedStaticMesh) (LocalVariables|GetTileTransform)))))))))))))

(fn GetShapeRowData
  (bind _grid_shape (Variables|Default|GetGrid%20Shape))
  (bind _returnvalue (Utilities|String|EnumtoString _grid_shape))
  (bind _returnvalue_2 (Utilities|GetDataTableRow "/Game/Blueprints/Core/Grid/Grid_Shapes/DT_Grid_Shape_Data.DT_Grid_Shape_Data" (Utilities|String|StringToName _returnvalue))
    (:then
      (return _returnvalue_2))
    (:RowNotFound
      (Development|PrintString (Utilities|String|Append "Error -cannot find row-" _returnvalue)))))

(fn DeleteGrid
  ;[1 1 1] 用于清理最初构建的基础实例，只留下spawned grid
  (Components|InstancedStaticMesh|ClearInstances (Variables|Default|GetInstancedStaticMesh)))

(fn CalCenter&BottomLeftLocation
  (bind _grid_tile_count (Variables|Default|GetGrid%20Tile%20Count))
  (switch Utilities|FlowControl|Switch|SwitchonE_Grid_Shape (Variables|Default|GetGrid%20Shape)
    (:NewEnumerator1
      ;[1 1 1] 将center的位置与网格点对齐，使移动grid时，grid始终在网格的边上
      (LocalVariables|SetCenter (CallFunction|SnapVectoVec (Variables|Default|GetGrid%20Center%20Location) (Variables|Default|GetGrid%20Tile%20Size)))
      (return (LocalVariables|GetCenter) (- (LocalVariables|GetCenter) (Math|Conversions|ToVector(Vector2D) (* (/ (- (Math|Conversions|ToVector2D(IntPoint) (Variables|Default|GetGrid%20Tile%20Count)) (Math|Vector2D|MakeVector2D (Math|Float|SelectFloat 0.0 1.0 (CallFunction|IsIntEven (.x _grid_tile_count))) (Math|Float|SelectFloat 0.0 1.0 (CallFunction|IsIntEven (.y _grid_tile_count))))) 2.0) (Math|Conversions|ToVector2D(Vector) (Variables|Default|GetGrid%20Tile%20Size)))))))
    (:NewEnumerator2
      ;[1 1 1] Hexagon:将center的位置与网格点对齐，使移动grid时，grid始终在网格的边上
      (LocalVariables|SetCenter (CallFunction|SnapVectoVec (Variables|Default|GetGrid%20Center%20Location) (* (Variables|Default|GetGrid%20Tile%20Size) "1.500000,1.000000,1.000000")))
      (return (LocalVariables|GetCenter) (- (LocalVariables|GetCenter) (CallFunction|SnapVectoVec (Math|Conversions|ToVector(Vector2D) (* (/ (Math|Conversions|ToVector2D(IntPoint) (Variables|Default|GetGrid%20Tile%20Count)) "(X=3.000000,Y=2.000000)") (Math|Conversions|ToVector2D(Vector) (Variables|Default|GetGrid%20Tile%20Size)))) (* (Variables|Default|GetGrid%20Tile%20Size) "1.500000,1.000000,1.000000")))))
    (:NewEnumerator3
      ;[1 1 1] Triangle:将center的位置与网格点对齐，使移动grid时，grid始终在网格的边上
      (LocalVariables|SetCenter (CallFunction|SnapVectoVec (Variables|Default|GetGrid%20Center%20Location) (* (Variables|Default|GetGrid%20Tile%20Size) "2.000000,1.000000,1.000000")))
      (return (LocalVariables|GetCenter) (- (LocalVariables|GetCenter) (CallFunction|SnapVectoVec (Math|Conversions|ToVector(Vector2D) (* (/ (- (Math|Conversions|ToVector2D(IntPoint) (Variables|Default|GetGrid%20Tile%20Count)) (Math|Vector2D|MakeVector2D 1.0 1.0)) "(X=2.000000,Y=4.000000)") (Math|Conversions|ToVector2D(Vector) (Variables|Default|GetGrid%20Tile%20Size)))) (* (Variables|Default|GetGrid%20Tile%20Size) "2.000000,1.000000,1.000000")))))))

(fn RotationBasedonGridIndex
  (params (GridIndex :type Int%20Point%20Structure))
  (if (Utilities|Enum|Equal(Enum) (Variables|Default|GetGrid%20Shape) "NewEnumerator3")
    (return (Math|Rotator|MakeRotator 0.0 0.0 (+ (Math|Float|SelectFloat 1.8e+02 0.0 (CallFunction|IsIntEven (.y GridIndex))) (Math|Float|SelectFloat 1.8e+02 0.0 (CallFunction|IsIntEven (.x GridIndex))))))
    (else
      (return "0, 0, 0"))))

(fn LocationBasedonGridIndex
  (params (Grid_Index :type Int%20Point%20Structure))
  (return (+ (Variables|Default|GetGridLeftBottomLocation) (* (Variables|Default|GetGrid%20Tile%20Size) (Math|Conversions|ToVector(Vector2D) (* (Math|Conversions|ToVector2D(IntPoint) Grid_Index) (Utilities|Select :Index (Variables|Default|GetGrid%20Shape) :NewEnumerator0 "" :NewEnumerator1 "(X=1.000000,Y=1.000000)" :NewEnumerator2 "(X=0.750000,Y=0.500000)" :NewEnumerator3 "(X=1.000000,Y=0.500000)")))))))

(fn TraceforGround
  (params (InLocation :type Vector))
  (Variables|Default|SetRadius (/ (.x (Variables|Default|GetGrid%20Tile%20Size)) (Math|Float|SelectFloat 5.0 3.0 (Utilities|Enum|Equal(Enum) (Variables|Default|GetGrid%20Shape) "NewEnumerator3"))))
  (bind _outhits (Collision|MultiSphereTraceByChannel (+ InLocation "0, 0,1000.000000") (- InLocation "0, 0,1000.000000") (Variables|Default|GetRadius) "TraceTypeQuery3" false 0 "None"))
  (if (> (Utilities|Array|Length _outhits) 0)
    (return (Math|Vector|MakeVector (.x InLocation) (.y InLocation) (Math|Float|SnapToGrid(Float) (- (.Z (Math|Vector|BreakVector (.Location (Collision|BreakHitResult (Utilities|Array|Get(acopy) _outhits))))) (Variables|Default|GetRadius)) (.z (Variables|Default|GetGrid%20Tile%20Size)))) true)
    (else
      (return InLocation false))))

(fn SetGridOffsetfromGround
  (params (Offset :type Float%20%28single-precision%29))
  (Variables|Default|SetGridOffsetFromGround Offset)
  (Transformation|SetWorldLocation (Variables|Default|GetInstancedStaticMesh) (Math|Vector|MakeVector 0.0 0.0 (Variables|Default|GetGridOffsetFromGround)) false false))