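; BP_Grid_Visual is the actor that renders a grid's walkable tiles as flat instanced meshes.
; It initializes a child BP_Grid_MeshInst with the flat mesh and material from the grid's shape data, using query-only collision.
; It sits at the world origin, raised by a ground offset, with tick disabled.
; Tile updates remove the old instance by index and re-add walkable tiles with their states.
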(event EventBeginPlay
  (Actor|Tick|SetActorTickEnabled false))

(event Collision|EventActorBeginOverlap
  (params (OtherActor :type Actor%20Object%20Reference)))

(event EventTick
  (params (DeltaSeconds :type Float%20%28single-precision%29)))

(fn ConstructionScript)

(fn InitializeGridVisual
  (params (Grid :type BP%20Grid%20Object%20Reference))
  (Variables|Default|SetGrid Grid)
  (bind _asbp_grid_mesh_inst (Utilities|Casting|CastToBP_Grid_MeshInst (Variables|/Script/Engine.ChildActorComponent|GetChildActor (Variables|Default|GetChildActor_GridMeshInst))))
  (Variables|Default|SetGrid_MeshInst _asbp_grid_mesh_inst)
  (Default|InitializeGridMeshInstance :self (Variables|Default|GetGrid_MeshInst) :Mesh (.FlatMesh (Utilities|Struct|BreakS_Grid_Shape_Data (Default|GetShapeRowData (Variables|Default|GetGrid)))) :Material (.FlatMetiral (Utilities|Struct|BreakS_Grid_Shape_Data (Default|GetShapeRowData (Variables|Default|GetGrid)))) :Collision "QueryOnly")
  (Transformation|SetActorLocation "0, 0, 0" false false) ; 真实世界的位置
  (CallFunction|SetOffestfromGround (Variables|Default|GetOffestFromGround)))

(fn SetOffestfromGround
  (params (Offest :type Float%20%28single-precision%29))
  (bind _returnvalue (Transformation|GetActorLocation))
  (Variables|Default|SetOffestFromGround Offest)
  (Transformation|SetActorLocation (Math|Vector|MakeVector (.x _returnvalue) (.y _returnvalue) (Variables|Default|GetOffestFromGround)) false false))

(fn DestoryGridVisual
  (bind _grid_meshinst (Variables|Default|GetGrid_MeshInst))
  (Utilities|IsValid _grid_meshinst
    (:Is%20Valid
      (Default|ClearInstance _grid_meshinst))))

(fn UpdateTileVisual
  (params (Data :type S%20Tile%20Data%20Structure))
  ;[1 1 1] 删除之前添加的实例，并用新的视觉效果，添加新的实例
  (Default|RemoveInstance (Variables|Default|GetGrid_MeshInst) (.index Data))
  (if (CallFunction|IsTileWakable (.type Data))
    (Default|InstanceAdd (Variables|Default|GetGrid_MeshInst) (.transform Data) (.index Data) (.states Data))))