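; BP_Actions turns player mouse input into tile hover, selection and pathfinding queries on BP_Grid, with debug visualization.
; Tick moves a hover state to the tile under the cursor.
; Left click toggles a single selection and draws spheres on neighbors within two steps.
; Right clicks alternately set source and destination, then run FindPath and draw the resulting path, clearing the previous pair's marks when a new source is picked.
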(event EventBeginPlay
  (bind _returnvalue (Actor|GetActorOfClass "/Game/Blueprints/Core/Grid/BP_Grid.BP_Grid_C"))
  (Variables|Default|SetGrid _returnvalue)
  (Input|EnableInput (Game|GetPlayerController 0)))

(event EventTick
  (params (DeltaSeconds :type Float%20%28single-precision%29))
  (CallFunction|UpdateTileUnderCursor))

(event Input|MouseEvents|LeftMouseButton
  (params (Key :type Key%20Structure :default "None"))
  (bind _hoveredtile (Variables|Default|GetHoveredTile))
  (:Pressed
    (bind _states (Default|GetTileState (Variables|Default|GetGrid) (Variables|Default|GetHoveredTile)))
    (if (>= (Utilities|Array|FindItem _states "NewEnumerator2") 0)
      (Default|RemoveStatefromTile (Variables|Default|GetGrid) (Variables|Default|GetHoveredTile) "NewEnumerator2")
      (else
        (Default|RemoveStatefromTile (Variables|Default|GetGrid) (Variables|Default|GetSelected_Tile) "NewEnumerator2")
        (Default|AddStatetoTile (Variables|Default|GetGrid) _hoveredtile "NewEnumerator2")
        (Variables|Default|SetSelected_Tile _hoveredtile)
        (for _array_element (Default|GetNeighborsinSteps (Variables|Default|GetGrid) (Variables|Default|GetHoveredTile) 2)
          (Development|PrintString (Utilities|String|ToString(Integer) _array_element))
          (Rendering|Debug|DrawDebugSphere (Default|LocationBasedonGridIndex (Variables|Default|GetGrid) _array_element) 1e+02 12 "(R=1.000000,G=1.000000,B=1.000000,A=1.000000)" 2.0))))))

(event Input|MouseEvents|RightMouseButton
  (params (Key :type Key%20Structure :default "None"))
  (bind _hoveredtile (Variables|Default|GetHoveredTile))
  (bind _grid (Variables|Default|GetGrid))
  (bind _hoveredtile_2 (Variables|Default|GetHoveredTile))
  (:Pressed
    (bind _states (Default|GetTileState (Variables|Default|GetGrid) (Variables|Default|GetHoveredTile)))
    (if (>= (Utilities|Array|FindItem _states "NewEnumerator2") 0)
      (Default|RemoveStatefromTile (Variables|Default|GetGrid) (Variables|Default|GetHoveredTile) "NewEnumerator2")
      (elif (!= (Variables|Default|GetSrc) (Utilities|Struct|MakeIntPoint -1 -1))
        (Default|AddStatetoTile (Variables|Default|GetGrid) _hoveredtile "NewEnumerator2")
        (Variables|Default|SetDst _hoveredtile)
        (bind _ispassable (Default|FindPath (Variables|Default|GetGrid) (Variables|Default|GetSrc) (Variables|Default|GetDst)))
        (if _ispassable
          (for _array_element (Variables|/Game/Blueprints/Core/Grid/BP_Grid.BP_Grid_C|GetPath _grid)
            (Rendering|Debug|DrawDebugSphere (Default|LocationBasedonGridIndex _grid _array_element) 1e+02 12 "(R=1.000000,G=0.000000,B=0.051075,A=1.000000)" 2.0)))
        (Variables|Default|SetPreSrc (Variables|Default|GetSrc))
        (Variables|Default|SetPreDst (Variables|Default|GetDst))
        (Variables|Default|SetSrc (Utilities|Struct|MakeIntPoint -1 -1))
        (Variables|Default|SetDst (Utilities|Struct|MakeIntPoint -1 -1))
        (else
          (Default|RemoveStatefromTile (Variables|Default|GetGrid) (Variables|Default|GetPreSrc) "NewEnumerator2")
          (Default|RemoveStatefromTile (Variables|Default|GetGrid) (Variables|Default|GetPreDst) "NewEnumerator2")
          (Default|AddStatetoTile (Variables|Default|GetGrid) _hoveredtile_2 "NewEnumerator2")
          (Variables|Default|SetSrc _hoveredtile_2))))))

(fn ConstructionScript)

(fn UpdateTileUnderCursor
  (bind _tileindex (Default|GetTileIndexonCursor (Variables|Default|GetGrid)))
  (if (!= _tileindex (Variables|Default|GetHoveredTile))
    (Default|RemoveStatefromTile (Variables|Default|GetGrid) (Variables|Default|GetHoveredTile) "NewEnumerator1")
    (Variables|Default|SetHoveredTile _tileindex)
    (Default|AddStatetoTile (Variables|Default|GetGrid) (Variables|Default|GetHoveredTile) "NewEnumerator1")))