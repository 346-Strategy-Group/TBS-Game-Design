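; Actor that switches between streaming sublevels by name, keeping track of the selected one in its Level variable.
; BeginPlay force-loads the initial Level.
; LoadLevel acts on a changed name or Force, clearing the previous level's ShouldBeLoaded and ShouldBeVisible flags, then storing and flagging the new one.
; It sets streaming flags directly and prints an error for unknown names other than "None".
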(event EventBeginPlay
  (CallFunction|LoadLevel (Variables|Default|GetLevel) true))

(event Collision|EventActorBeginOverlap
  (params (OtherActor :type Actor%20Object%20Reference)))

(event EventTick
  (params (DeltaSeconds :type Float%20%28single-precision%29)))

(fn ConstructionScript)

(fn LoadLevel
  (params (Level :type String) (Force :type Boolean))
  ;[1 1 1] 判断是否需要加载关卡
  (if (or Force (Utilities|Enum|NotEqual(Enum) Level (Variables|Default|GetLevel)))
    (Utilities|FlowControl|Sequence
      (:then_0
        ;[1 1 1] 取消之前关卡的加载
        (Utilities|IsValid (Class|GameplayStatics|GetStreamingLevel (Utilities|String|StringToName (Variables|Default|GetLevel)))
          (:Is%20Valid
            (Variables|/Script/Engine.LevelStreaming|SetbShouldBeLoaded (Class|GameplayStatics|GetStreamingLevel (Utilities|String|StringToName (Variables|Default|GetLevel))) false)
            (Variables|/Script/Engine.LevelStreaming|SetbShouldBeVisible (Class|GameplayStatics|GetStreamingLevel (Utilities|String|StringToName (Variables|Default|GetLevel))) false))))
      (:then_1
        ;[1 1 1] 加载当前选定关卡
        (bind _output_get (Variables|Default|SetLevel Level))
        (Utilities|IsValid (Class|GameplayStatics|GetStreamingLevel (Utilities|String|StringToName _output_get))
          (:Is%20Valid
            (Variables|/Script/Engine.LevelStreaming|SetbShouldBeLoaded (Class|GameplayStatics|GetStreamingLevel (Utilities|String|StringToName _output_get)) true)
            (Variables|/Script/Engine.LevelStreaming|SetbShouldBeVisible (Class|GameplayStatics|GetStreamingLevel (Utilities|String|StringToName _output_get)) true))
          (:Is%20Not%20Valid
            (if (Utilities|Enum|NotEqual(Enum) (Variables|Default|GetLevel) "None")
              (Development|PrintString (Utilities|String|Append "Error-Load  Invalid Level name-" (Variables|Default|GetLevel))))))))))