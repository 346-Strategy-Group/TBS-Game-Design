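; BP_Hero is a hero Blueprint whose HeroType selects its skeletal mesh and animation class in the construction script, with only Warrior mapped.
; BeginPlay sends a test animation state to the anim instance through an interface message.
; MoveByGrid stores the grid and source and destination nodes, then branches on grid shape with empty cases, leaving movement unimplemented and its location math unconnected.
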(event EventBeginPlay
  (Variables|Default|SetTestAnimIndex "NewEnumerator0")
  (Class|BPIHeroAnimation|SetHeroAnimationStates(Message) (Components|SkeletalMesh|GetAnimInstance (Variables|Default|GetSkeletalMesh)) (Variables|Default|GetTestAnimIndex)))

(event Collision|EventActorBeginOverlap
  (params (OtherActor :type Actor%20Object%20Reference)))

(event EventTick
  (params (DeltaSeconds :type Float%20%28single-precision%29)))

(fn ConstructionScript
  (bind _skeletalmesh (Variables|Default|GetSkeletalMesh))
  (Class|SkinnedMeshComponent|SetSkeletalMesh _skeletalmesh (Utilities|Select :Index (Variables|Default|GetHeroType) :NewEnumerator0 "/Game/Art/Heros/Warrior/SK_Warrior.SK_Warrior") true)
  (Class|SkeletalMeshComponent|SetAnimClass _skeletalmesh (Utilities|Select :Index (Variables|Default|GetHeroType) :NewEnumerator0 "/Game/Art/Heros/Warrior/ABP_Warrior.ABP_Warrior_C")))

(fn MovebyGrid
  (params (Grid :type BP%20Grid%20Object%20Reference) (src :type Int%20Point%20Structure) (dst :type Int%20Point%20Structure))
  (LocalVariables|SetFromNode src)
  (LocalVariables|SetToNode dst)
  (Variables|Default|SetGrid Grid)
  (switch Utilities|FlowControl|Switch|SwitchonE_Grid_Shape (Variables|/Game/Blueprints/Core/Grid/BP_Grid.BP_Grid_C|GetGrid%20Shape Grid)))